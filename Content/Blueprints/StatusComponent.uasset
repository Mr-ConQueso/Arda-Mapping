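; StatusComponent is a component that holds current health and stamina values and provides functions to reduce them.
; DecreaseStamina and DecreaseHealth each subtract an amount and clamp the result at zero.
; DecreaseHealth also returns a below-zero check, which repeats the subtraction on the already reduced health rather than testing the original value.
; The event graph has no active logic, so changes happen only through these function calls.
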(fn `DecreaseHealth`
  (params (Amount :type "Float (double-precision)"))
  (returns (IsDead :type Boolean))
  (bind _returnvalue (- (`self.CurrentHealth`) Amount))
  (bind _returnvalue_2 (< _returnvalue 0.0))
  (set `self.CurrentHealth` (select `bool` _returnvalue_2 :`false` _returnvalue))
  (return _returnvalue_2))

(fn `DecreaseStamina`
  (params (Amount :type "Float (double-precision)"))
  (bind _returnvalue (- (`self.CurrentStamina`) Amount))
  (set `self.CurrentStamina` (select `bool` (< _returnvalue 0.0) :`false` _returnvalue))
  (return))