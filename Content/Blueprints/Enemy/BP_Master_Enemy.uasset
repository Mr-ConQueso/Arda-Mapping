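; Base enemy Blueprint that handles taking damage, showing health and reacting to hits.
; ReciveDamage lowers health through StatusComponent and refreshes the HP bar widget cached on BeginPlay.
; It then destroys the actor if DecreaseHealth returns true, otherwise plays a hit montage from GetHitAnimation.
; GetHitAnimation sorts the attacker's relative yaw into front, back, left or right, though no branch shows an assigned montage.
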(event `/Game/Blueprints/I_Interactions.ReciveDamage`
  (params (DamageAmount :type "Float (double-precision)") (AttackingActor :type "Actor Object Reference"))
  (bind _isdead (`/Game/Blueprints/StatusComponent.DecreaseHealth` (`self.StatusComponent`) DamageAmount))
  (`/Game/Widgets/WBP_HPBar.RefreshHealthBar` (`self.WBPHPBar`) (`self.StatusComponent`))
  (if _isdead
    (`self.K2_DestroyActor`)
    (else
      (`self.PlayAnimMontage` (`self.GetHitAnimation` AttackingActor)))))

(event `self.ReceiveBeginPlay`
  ;[1 0.5717 0.2314] Init
  ;;[0.02452 0.02998 0.05098] Refresh Health Bar
  (bind _output_get (set `self.WBPHPBar` (cast `/Game/Widgets/WBP_HPBar` (`WidgetComponent.GetUserWidgetObject` (`self.HealthBar`)) :!pure true)))
  (`/Game/Widgets/WBP_HPBar.RefreshHealthBar` _output_get (`self.StatusComponent`)))

(fn `GetHitAnimation`
  (params (AtackingActor :type "Actor Object Reference"))
  (returns (Animation :type "AnimMontage Object Reference"))
  (bind (_returnvalue_roll _returnvalue_pitch _returnvalue_yaw) (`KismetMathLibrary.BreakRotator` (`KismetMathLibrary.NormalizedDeltaRotator` (`self.K2_GetActorRotation`) (`KismetMathLibrary.FindLookAtRotation` (`self.K2_GetActorLocation`) (`self.K2_GetActorLocation` AtackingActor)))))
  (switch `/Game/Blueprints/E_HitAngle` (select `bool` (`KismetMathLibrary.InRange_FloatFloat` _returnvalue_yaw -45.0 45.0) :`false` (select `bool` (or (`KismetMathLibrary.InRange_FloatFloat` _returnvalue_yaw -180.0 -135.0) (`KismetMathLibrary.InRange_FloatFloat` _returnvalue_yaw 135.0 180.0)) :`false` (select `bool` (`KismetMathLibrary.InRange_FloatFloat` _returnvalue_yaw 46.0 134.0) :`false` (select `bool` (`KismetMathLibrary.InRange_FloatFloat` _returnvalue_yaw -134.0 -46.0) :`false` "NewEnumerator0" :`true` "NewEnumerator3" :!type "/Game/Blueprints/E_HitAngle Enum") :`true` "NewEnumerator2") :`true` "NewEnumerator1") :`true` "NewEnumerator0")
    (:`NewEnumerator0`
      (return null))
    (:`NewEnumerator1`
      (return null))
    (:`NewEnumerator2`
      (return null))
    (:`NewEnumerator3`
      (return null))))

(fn `UserConstructionScript`)